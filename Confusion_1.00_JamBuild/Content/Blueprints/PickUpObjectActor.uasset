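; Pickup object actor that floats upward and shows a widget while the player is inside its collision sphere, then sinks back down when they leave.
; Two timelines lerp between positions set in the construction script from the placed location.
; State flags gate the timelines, and Tick corrects the height if the player enters or leaves mid-animation.
; A looping timer yaws the widget to face the player.
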(event `self.ReceiveBeginPlay`
  (`|ExecutionSequence`
    (:`then_0`
      (bind _asfirst_person_character (cast `/Game/Blueprints/FirstPersonCharacter` (`GameplayStatics.GetPlayerPawn` 0)))
      (set `self.Player Ref` _asfirst_person_character)
      (`SceneComponent.SetVisibility` (`self.Widget`) false false))
    (:`then_1`
      (`KismetSystemLibrary.K2_SetTimerDelegate` (delegate `Spin`) 0.016667 true))))

(event `Spin`
  (bind _widget (`self.Widget`))
  (bind (_returnvalue_roll _returnvalue_pitch _returnvalue_yaw) (`KismetMathLibrary.BreakRotator` (`KismetMathLibrary.FindLookAtRotation` (`SceneComponent.K2_GetComponentLocation` _widget) (`SceneComponent.K2_GetComponentLocation` (`Character.CapsuleComponent` (`self.Player Ref`))))))
  (`SceneComponent.K2_SetWorldRotation` _widget (`KismetMathLibrary.MakeRotator` 0.0 0.0 _returnvalue_yaw) false false))

(event `self.Sphere Collision.OnComponentBeginOverlap`
  (params (OverlappedComponent :type "PrimitiveComponent Object Reference") (OtherActor :type "Actor Object Reference") (OtherComp :type "PrimitiveComponent Object Reference") (OtherBodyIndex :type Integer) (bFromSweep :type Boolean) (SweepResult :type "HitResult Structure (by ref)"))
  (if (== OtherActor (`self.Player Ref`))
    (`SceneComponent.SetVisibility` (`self.Widget`) true false)
    (`|ExecutionSequence`
      (:`then_0`
        (if (and (and (not (`self.Can Interact`)) (`self.Timelines Finished`)) (not (`self.ObjectUp`)))
          (set `self.Timelines Finished` false :!label _label)
          (bind (_direction _newtrack_0) (`Timeline|FloatUp` :!via `PlayFromStart`)
            (:`Update`
              (`self.K2_SetActorLocation` self (`KismetMathLibrary.VLerp` (`self.floatDownLocation`) (`self.floatUpLocation`) _newtrack_0) false false))
            (:`Finished`
              (set `self.Timelines Finished` true)
              (set `self.ObjectUp` true)))))
      (:`then_1`
        (set `self.Can Interact` true)))))

(event `self.ReceiveTick`
  (params (DeltaSeconds :type "Float (single-precision)"))
  ;[1 1 1] Event tick to ensure that the object is correctly floating. Necessary since the character could leave before the timelines finish
  (if (and (and (`self.Can Interact`) (`self.Timelines Finished`)) (not (`self.ObjectUp`)))
    (goto _label)
    (elif (and (and (not (`self.Can Interact`)) (`self.Timelines Finished`)) (`self.ObjectUp`))
      (set `self.Timelines Finished` false :!label _label_2)
      (bind (_direction _newtrack_0) (`Timeline|FloatDown` :!via `ReverseFromEnd`)
        (:`Update`
          (`self.K2_SetActorLocation` self (`KismetMathLibrary.VLerp` (`self.floatDownLocation`) (`self.floatUpLocation`) _newtrack_0) false false))
        (:`Finished`
          (set `self.Timelines Finished` true)
          (set `self.ObjectUp` false))))))

(event `self.Sphere Collision.OnComponentEndOverlap`
  (params (OverlappedComponent :type "PrimitiveComponent Object Reference") (OtherActor :type "Actor Object Reference") (OtherComp :type "PrimitiveComponent Object Reference") (OtherBodyIndex :type Integer))
  (if (== (`self.Player Ref`) OtherActor)
    (`SceneComponent.SetVisibility` (`self.Widget`) false false)
    (`|ExecutionSequence`
      (:`then_0`
        (if (and (and (`self.Can Interact`) (`self.Timelines Finished`)) (`self.ObjectUp`))
          (goto _label_2)))
      (:`then_1`
        (set `self.Can Interact` false)))))

(fn `UserConstructionScript`
  (bind _returnvalue (`self.K2_GetActorLocation` self))
  (set `self.floatDownLocation` _returnvalue)
  (set `self.floatUpLocation` (+ _returnvalue (0.0 0.0 215.0))))